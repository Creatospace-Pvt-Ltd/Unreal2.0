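; Interactable in-world screen that displays a screen share on its front and back planes.
; Interacting requests ownership for the character and opens the screenshare widget; resetting releases ownership and closes it.
; Owner-checked activation plays a screencap:// stream through a runtime-built MediaPlayer into a MediaTexture on a dynamic material.
; Stopping clears the stream URL and restores the black material; the MULTI events are empty stubs.
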(event `self.ReceiveBeginPlay`
  (`|ExecutionSequence`
    (:`then_0`
      (`self.InitializeResources`))))

(event `/Game/Creatospace/Blueprints/Interfaces/InteractInterface.Interact_E`
  (params (`Actor Ref` :type "Actor Object Reference") (`Component Ref` :type "PrimitiveComponent Object Reference"))
  ;[0 0.01135 0.1248] Interact : Start & Stop Screen Share
  (`|ExecutionSequence`
    (:`then_0`
      (bind _asbp_rpm_third_person_char (cast `/Game/Creatospace/Blueprints/BP_RPM_ThirdPersonChar` `Actor Ref`))
      (`/Game/Creatospace/Blueprints/BP_RPM_ThirdPersonChar.Update Owner SERVER` _asbp_rpm_third_person_char self _asbp_rpm_third_person_char))
    (:`then_1`
      (bind _output_get (set `self.CurrentInteractingActor` `Actor Ref`))
      (bind _asbp_rpm_third_person_char_2 (cast `/Game/Creatospace/Blueprints/BP_RPM_ThirdPersonChar` _output_get))
      (`KismetSystemLibrary.PrintString` "ScreenWidget Open")
      (bind _current_player_controller (`/Game/Creatospace/Blueprints/BP_RPM_ThirdPersonChar.Current Player Controller` _asbp_rpm_third_person_char_2))
      (bind _returnvalue (`|CreateWidget` "/Game/Creatospace/Widgets/Screen_Share/WBP_ScreenshareWidget.WBP_ScreenshareWidget_C" _current_player_controller))
      (bind _output_get_2 (set `self.ScreenShareWidget` _returnvalue))
      (set `/Game/Creatospace/Widgets/Screen_Share/WBP_ScreenshareWidget.ScreenShareActorRef` self _output_get_2)
      (`WidgetBlueprintLibrary.SetInputMode_GameAndUIEx` _current_player_controller _returnvalue)
      (`UserWidget.AddToViewport` _output_get_2 0)
      (`Widget.SetVisibility` _output_get_2 "Visible"))))

(event `/Game/Creatospace/Blueprints/Interfaces/InteractInterface.ResetInteraction`
  ;[0 0.01135 0.1248] Interact : Start & Stop Screen Share
  (`|ExecutionSequence`
    (:`then_0`
      (bind _asbp_rpm_third_person_char (cast `/Game/Creatospace/Blueprints/BP_RPM_ThirdPersonChar` (`self.CurrentInteractingActor`)))
      (`/Game/Creatospace/Blueprints/BP_RPM_ThirdPersonChar.Update Owner SERVER` _asbp_rpm_third_person_char self null))
    (:`then_1`
      (`KismetSystemLibrary.PrintString` "Hello" true true (struct :`R` 0.012983 :`G` 0.023153 :`B` 0.124772 :`A` 1.0) 10.0)
      (bind _screensharewidget (`self.ScreenShareWidget`)
        (:`then`
          (`/Game/Creatospace/Widgets/Screen_Share/WBP_ScreenshareWidget.StopSharingScreen` _screensharewidget)
          (`Widget.RemoveFromParent` _screensharewidget))
        (:`else`)))))

(event `InitializeResources`
  (bind _mediatexture (`self.MediaTexture`))
  (bind _returnvalue (`|GenericCreateObject` self "/Script/MediaAssets.StreamMediaSource"))
  (bind _output_get (set `self.ScreenStreamSource` _returnvalue))
  (bind _returnvalue_2 (`|GenericCreateObject` self "/Script/MediaAssets.MediaPlayer"))
  (bind _output_get_2 (set `self.MediaPlayer` _returnvalue_2))
  (`MediaPlayer.SetMediaOptions` _output_get_2 _output_get)
  (`MediaPlayer.OpenSource` (`self.MediaPlayer`) (`self.ScreenStreamSource`))
  (set `MediaTexture.NewStyleOutput` false _mediatexture)
  (set `MediaTexture.OutputFormat` "MTOF_Default" _mediatexture)
  (`MediaTexture.UpdateResource` _mediatexture)
  (`MediaTexture.SetMediaPlayer` _mediatexture (`self.MediaPlayer`)))

(event `ActivateMedia`
  (bind _mediaplayer (`self.MediaPlayer`))
  (bind _screenstreamsource (`self.ScreenStreamSource`))
  (`KismetSystemLibrary.PrintString` "Trying activate screenshare" true true (struct :`A` 1.0))
  (set `StreamMediaSource.StreamUrl` "screencap://0?fps=60&capture_cursor=true" _screenstreamsource)
  (`MediaPlayer.SetMediaOptions` _mediaplayer _screenstreamsource)
  (`MediaPlayer.OpenSourceWithOptions` _mediaplayer _screenstreamsource (make `MediaPlayerOptions` (struct :`Caption` -1 :`Metadata` -1 :`Script` -1 :`Subtitle` -1 :`Text` -1) "+00000000.00:00:00.000000000" (`self.Play On Open`) (`self.Loop`)))
  (`MediaSoundComponent.SetMediaPlayer` (`self.MediaSound`) _mediaplayer))

(event `ActivateScreenSharing SERVER`
  (params (`WBP Screenshare Ref` :type "/Game/Creatospace/Widgets/Screen_Share/WBP_ScreenshareWidget Object Reference") (`Calling Actor Ref` :type "Actor Object Reference"))
  (bind _mediatexture (`self.MediaTexture`))
  (if (== `Calling Actor Ref` (`self.GetOwner`))
    (`KismetSystemLibrary.PrintString` "Owner Verified" true true (struct :`R` 0.021304 :`G` 0.251042 :`A` 1.0) 4.0)
    (bind _returnvalue (`PrimitiveComponent.CreateDynamicMaterialInstance` (`self.Plane`) 0 (`self.Source Material`) "None"))
    (set `self.Dyn Media Mat` _returnvalue)
    (`MediaTexture.UpdateResource` _mediatexture)
    (`MaterialInstanceDynamic.SetTextureParameterValue` (`self.Dyn Media Mat`) "Texture" _mediatexture)
    (`PrimitiveComponent.SetMaterial` (`self.Plane`) 0 (`self.Dyn Media Mat`))
    (`PrimitiveComponent.SetMaterial` (`self.Back`) 0 (`self.Dyn Media Mat`))
    (`self.ActivateMedia`)
    (else
      (`KismetSystemLibrary.PrintString` (`KismetStringLibrary.Concat_StrStr` "Not the owner, screen not shared: " (`KismetSystemLibrary.GetObjectName` `Calling Actor Ref`)) true true (struct :`R` 1.0 :`G` 0.067656 :`A` 1.0) 4.0))))

(event `ActivateScreenSharing MULTI`)

(event `StopScreenSharing SERVER`
  (params (`WBP Screenshare Ref` :type "/Game/Creatospace/Widgets/Screen_Share/WBP_ScreenshareWidget Object Reference"))
  (set `StreamMediaSource.StreamUrl` "" (`self.ScreenStreamSource`))
  (`MediaTexture.UpdateResource` (`self.MediaTexture`))
  (`PrimitiveComponent.SetMaterial` (`self.Plane`) 0 "/Game/Creatospace/Assets/MemeStreet/pepe-the-frog/source/Black.Black")
  (`PrimitiveComponent.SetMaterial` (`self.Back`) 0 "/Game/Creatospace/Assets/MemeStreet/pepe-the-frog/source/Black.Black"))

(event `StopScreenSharing MULTI`)

(fn `UserConstructionScript`)