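; Multiplayer player controller handling dedicated-server sessions, EOS voice chat, text chat and avatar configuration UI.
; Session events accept the player, find, join or create an EOS session, and on exit remove the player, terminating when one controller remains.
; Voice fetches a room token over HTTP using the GameInstance access token, then reuses LoginWithEOS to join and mute.
; Chat messages go to GameState; the avatar-generated callback is an empty stub.
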(event `GetRoomTokenWeb`
  (params (PUID :type String) (IP :type String) (RoomID :type String))
  (`KismetSystemLibrary.PrintString` (`KismetStringLibrary.Concat_StrStr` "PUID:" PUID "IP:" IP))
  (bind _asbp_mpgame_instance (cast `/Game/Creatospace/Blueprints/BP_MPGameInstance` (`GameplayStatics.GetGameInstance`)))
  (bind _tokenexpirydatetime (`/Game/Creatospace/Blueprints/BP_MPGameInstance.TokenExpiryDateTime` _asbp_mpgame_instance))
  (if (`KismetStringLibrary.NotEqual_StrStr` _tokenexpirydatetime)
    (bind (_result _returnvalue) (`KismetMathLibrary.DateTimeFromIsoString` _tokenexpirydatetime))
    (if _returnvalue
      (if (<= (`KismetMathLibrary.UtcNow`) _result)
        (`HTTPRequestClient.MakeAHttpRequest` "POST" "" (`|MakeMap` "") (`|MakeMap` "Authorization" (`KismetStringLibrary.Concat_StrStr` "Bearer " (`/Game/Creatospace/Blueprints/BP_MPGameInstance.AccessToken` _asbp_mpgame_instance)) "Content-Type" "application/json" "Accept" "application/json") (`KismetStringLibrary.Concat_StrStr` "{ \"participants\": [ { \"puid\": \"" PUID "\",\"clientIp\": \"" IP "\", \"hardMuted\": false } ] }") (delegate `OnConnectSuccess`))
        (else
          (`KismetSystemLibrary.Delay` 2.0 :!label _label)
          (`self.GetRoomTokenWeb` PUID IP RoomID))))
    (else
      (goto _label))))

(event `OnConnectSuccess`
  (params (Status :type Byte) (ResponseString :type String))
  (bind _returnvalue (`BlueprintJsonLibrary.Conv_StringToJsonObject` ResponseString))
  (bind _returnvalue_2 (`BlueprintJsonLibrary.Conv_JsonValueToString` (`BlueprintJsonLibrary.Conv_JsonObjectToJsonValue` _returnvalue "clientBaseUrl")))
  (bind _returnvalue_3 (`BlueprintJsonLibrary.Conv_JsonValueToString` (`BlueprintJsonLibrary.Conv_JsonObjectToJsonValue` (`BlueprintJsonLibrary.Conv_JsonValueToObject` (`|GetArrayItem` (`BlueprintJsonLibrary.Conv_JsonValueToArray` (`BlueprintJsonLibrary.Conv_JsonObjectToJsonValue` _returnvalue "participants")))) "token")))
  (if (== Status 200)
    (`KismetSystemLibrary.PrintString` ResponseString)
    (`KismetSystemLibrary.PrintString` "Hello")
    (`KismetSystemLibrary.PrintString` "Hello")
    (set `self.VoiceToken` _returnvalue_3)
    (set `self.ClientBaseUrl` _returnvalue_2)
    (`self.Client join voice` _returnvalue_2 _returnvalue_3 (stale `GetRoomTokenWeb` PUID) (stale `GetRoomTokenWeb` RoomID))
    (else
      (`KismetSystemLibrary.PrintString` ResponseString))))

(event `set Room id`
  (params (`Room ID` :type String))
  (set `self.Room ID` `Room ID`))

(event `set Map name`
  (params (`map name` :type String))
  (set `self.Map Name` `map name`))

(event `Set Server IP`
  (params (`Server IP` :type String))
  (set `self.Server IP` `Server IP`))

(event `Start Voice`
  (bind _asbp_mpgame_instance (cast `/Game/Creatospace/Blueprints/BP_MPGameInstance` (`GameplayStatics.GetGameInstance`)))
  (bind _returnvalue (`One_Click_EOS_Subsystem.getPUID` (subsystem `One_Click_EOS_Subsystem`)))
  (`self.GetRoomTokenWeb` _returnvalue (`/Game/Creatospace/Blueprints/BP_MPGameInstance.IP` _asbp_mpgame_instance) (`/Game/Creatospace/Blueprints/BP_MPGameInstance.Room ID` _asbp_mpgame_instance)))

(event `Print on client`
  (params (String :type String))
  (`KismetSystemLibrary.PrintString` (`KismetStringLibrary.Concat_StrStr` "Print from server: " String)))

(event `Accept my client`
  (params (`Client session id` :type String))
  (`self.AcceptClient` `Client session id`)
  (`self.Print on client` `Client session id`))

(event `Server session find`
  (bind _returnvalue (`GameplayStatics.GetPlayerController` 0))
  ;[1 1 1] Find sessions
  (`/Engine/EditorBlueprintResources/StandardMacros.IsValid` (`self.PlayerState`)
    (:`Is Valid`
      (`KismetSystemLibrary.Delay` 1.0))
    (:`Is Not Valid`
      (bind _asbp_mpgame_instance (cast `/Game/Creatospace/Blueprints/BP_MPGameInstance` (`GameplayStatics.GetGameInstance`)))
      (bind _playersession_id (`/Game/Creatospace/Blueprints/BP_MPGameInstance.PlayerSession ID` _asbp_mpgame_instance))
      (`KismetSystemLibrary.PrintString` _playersession_id)
      (set `self.Player Session ID` _playersession_id)
      (`self.Accept my client` _playersession_id)
      (`self.set Room id` (`/Game/Creatospace/Blueprints/BP_MPGameInstance.Room ID` _asbp_mpgame_instance))
      (`self.set Map name` (`/Game/Creatospace/Blueprints/BP_MPGameInstance.Map Name` _asbp_mpgame_instance))
      (`self.Set Server IP` (`/Game/Creatospace/Blueprints/BP_MPGameInstance.Server IP Address` _asbp_mpgame_instance))
      (`/Engine/EditorBlueprintResources/StandardMacros.IsValid` _returnvalue :!label _label_2
        (:`Is Valid`
          (`KismetSystemLibrary.Delay` 1.0)
          (bind _results (`FindSessionsCallbackProxyAdvanced.FindSessionsAdvanced` :`PlayerController` _returnvalue :`MaxResults` 10 :`ServerTypeToSearch` "DedicatedServersOnly" :`bSearchLobbies` false)
            (:`OnSuccess`
              (bind _output (`|GetArrayItem` _results))
              (bind _sessionid (`AdvancedSessionsLibrary.GetSessionID_AsString` _output))
              (`KismetSystemLibrary.PrintString` (`KismetStringLibrary.Concat_StrStr` "Server sessions from Game Instance: " _sessionid))
              (if (`KismetStringLibrary.EqualEqual_StrStr` _sessionid)
                (`self.Server session create`)
                (else
                  (`self.Joinsessionas client` _output))))))
        (:`Is Not Valid`
          (goto _label_2))))))

(event `Load Widgets`
  (bind _returnvalue (`GameplayStatics.GetPlayerController` 0))
  (if (`KismetSystemLibrary.IsDedicatedServer`)
    (`/Engine/EditorBlueprintResources/StandardMacros.IsValid` _returnvalue :!label _label_3
      (:`Is Valid`
        (bind _returnvalue_2 (`|CreateWidget` "/Game/Creatospace/Widgets/WBP_ChatBox.WBP_ChatBox_C" _returnvalue))
        ;[1 1 1] For Avatar change
        (bind _output_get (set `self.ChatBoxWidget` _returnvalue_2))
        (`UserWidget.AddToViewport` _output_get 0)
        (`Widget.SetVisibility` (`self.ChatBoxWidget`) "Hidden"))
      (:`Is Not Valid`
        (`KismetSystemLibrary.Delay` 1.0)
        (goto _label_3)))))

(event `Joinsessionas client`
  (params (`Search result` :type "BlueprintSessionResult Structure"))
  (bind _returnvalue (`GameplayStatics.GetPlayerController` 0))
  ;[1 1 1] Find sessions
  (`/Engine/EditorBlueprintResources/StandardMacros.IsValid` _returnvalue :!label _label_4
    (:`Is Valid`
      (`JoinSessionCallbackProxy.JoinSession` _returnvalue `Search result`
        (:`OnSuccess`
          (`KismetSystemLibrary.PrintString` "Joined session" true true (struct :`R` 0.043207 :`G` 1.0 :`A` 1.0)))
        (:`OnFailure`
          (`KismetSystemLibrary.PrintString` "Failed to join session" true true (struct :`R` 1.0 :`G` 0.131859 :`B` 0.107983 :`A` 1.0))
          (`self.Server session create`))))
    (:`Is Not Valid`
      (`KismetSystemLibrary.Delay` 1.0)
      (goto _label_4))))

(event `Client join voice`
  (params (url :type String) (Token :type String) (PUID :type String) (RoomID :type String))
  (bind _returnvalue (subsystem `One_Click_EOS_Subsystem`))
  (bind _returnvalue_2 (`One_Click_EOS_Subsystem.getPUID` _returnvalue))
  (if (`KismetStringLibrary.EqualEqual_StrStr` PUID _returnvalue_2)
    (`One_Click_EOS_Subsystem.Login_With_EOS` _returnvalue url Token RoomID)
    (`KismetSystemLibrary.Delay` 2.0)
    (`One_Click_EOS_Subsystem.Login_With_EOS` _returnvalue RoomID "" "registerNotif")))

(event `self.ReceiveBeginPlay`
  ;[1 1 1] For Avatar change
  (bind _returnvalue (`|CreateWidget` "/Game/Creatospace/Widgets/WBP_AvatarConfig.WBP_AvatarConfig_C" (`GameplayStatics.GetPlayerController` 0)))
  (set `self.WBP_AvatarConfig` _returnvalue)
  (cast `/Game/Creatospace/Blueprints/BP_RPM_ThirdPersonChar` (`self.K2_GetPawn` (`GameplayStatics.GetPlayerController` 0)))
  (add `/Game/Creatospace/Widgets/WBP_AvatarConfig.AvatarGeneratedEvent` (`self.WBP_AvatarConfig`) (delegate `CallAvatarLoadServer`)))

(event `CallAvatarLoadServer`
  (params (AvatarUrl :type String))
  ;[1 1 1] For Avatar change
)

(event `Mute`
  (bind _asbp_mpgame_instance (cast `/Game/Creatospace/Blueprints/BP_MPGameInstance` (`GameplayStatics.GetGameInstance`)))
  (`One_Click_EOS_Subsystem.Login_With_EOS` (subsystem `One_Click_EOS_Subsystem`) (`/Game/Creatospace/Blueprints/BP_MPGameInstance.Room ID` _asbp_mpgame_instance) "mute" "localMute"))

(event `OpenChatSystem`
  (bind _chatboxwidget (`self.ChatBoxWidget`))
  (if (`self.Is Chat Visible`)
    (`Widget.SetVisibility` _chatboxwidget "Hidden")
    (set `self.Is Chat Visible` false)
    (else
      (`Widget.SetVisibility` _chatboxwidget "Visible")
      (set `self.Is Chat Visible` true))))

(event `Unmute`
  (bind _asbp_mpgame_instance (cast `/Game/Creatospace/Blueprints/BP_MPGameInstance` (`GameplayStatics.GetGameInstance`)))
  (`One_Click_EOS_Subsystem.Login_With_EOS` (subsystem `One_Click_EOS_Subsystem`) (`/Game/Creatospace/Blueprints/BP_MPGameInstance.Room ID` _asbp_mpgame_instance) "unmute" "localMute"))

(event `Server session create`
  ;[1 1 1] Create Dedicated Server Session
  (`One_Click_EOS_Subsystem.Create_EOS_Session` (subsystem `One_Click_EOS_Subsystem`) true false false 50 3 false false false false false true false (`KismetStringLibrary.Concat_StrStr` "/Game/Maps/" (`self.Map Name`)))
  (`self.Print on client` "OOOOO::: Advanced Session Created by server!!!!! OOOOO"))

(event `Server AddMessage`
  (params (Message :type Text))
  (bind _asbp_game_state (cast `/Game/Creatospace/Blueprints/BP_GameState` (`GameplayStatics.GetGameState`)))
  (bind _asbp_player_state (cast `/Game/Creatospace/Blueprints/BP_PlayerState` (`GameplayStatics.GetPlayerState` 0)))
  (`/Game/Creatospace/Blueprints/BP_GameState.AddMessage` _asbp_game_state (make `/Game/Creatospace/Widgets/SMessageData` (`/Game/Creatospace/Blueprints/BP_PlayerState.DisplayName` _asbp_player_state) Message)))

(event `Client travel called from server`
  (params (Map :type String))
  (`GameplayStatics.OpenLevel` (`KismetStringLibrary.Conv_StringToName` Map)))

(event `End Server session`
  (params (`Player Session ID` :type String))
  (bind _returnvalue (`GameplayStatics.GetNumPlayerControllers`))
  (`self.Print on client` (`KismetStringLibrary.Conv_IntToString` _returnvalue))
  (if (== _returnvalue 1)
    (`EndSessionCallbackProxy.EndSession` (`GameplayStatics.GetPlayerController` 0)
      (:`then`
        (`self.Client travel called from server` (`KismetStringLibrary.Concat_StrStr` "/Game/Maps/" "Server" "?listen"))
        (`self.RemovePlayerSession` `Player Session ID`)
        (`self.TerminateGameSession`)))
    (else
      (`self.Client travel called from server` "Lobby")
      (`self.RemovePlayerSession` `Player Session ID`))))

(fn `UserConstructionScript`)