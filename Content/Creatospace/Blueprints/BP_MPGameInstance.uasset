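; Multiplayer game instance that handles Epic Online Services sign-in and server travel for Creatospace.
; On Init it looks up the public IP, then dedicated servers fetch an EOS token with hardcoded credentials, while others log in by device ID and poll until ready.
; EnterMP_Server posts a room ID to an AWS session endpoint and opens the returned IP:port.
; GoToLevel opens listen-server maps by name; GetServerIPAddress holds only empty placeholder addresses.
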(event `GetAccessToken`
  (`HTTPRequestClient.MakeAHttpRequest` "POST" "https://api.epicgames.dev/auth/v1/oauth/token" (`|MakeMap` "") (`|MakeMap` "Authorization" "Basic eHl6YTc4OTFBNURoUkZXeEx5RUhsamdteVVnOUpXcnM6dTF4QUQyRUkxV2lTVkpuRjJWM1hrMERORGpjUGFvUmtqZlBSTmVLc3g2OA==" "Content-Type" "application/x-www-form-urlencoded" "Accept" "application/json") (`KismetStringLibrary.Concat_StrStr` "grant_type=" "client_credentials&" "deployment_id=" "8e95a37730924f708acb27dd265db81d") (delegate `OnConnectSuccess`)))

(event `OnConnectSuccess`
  (params (Status :type Byte) (ResponseString :type String))
  (bind _returnvalue (`BlueprintJsonLibrary.Conv_StringToJsonObject` ResponseString))
  (bind _returnvalue_2 (`BlueprintJsonLibrary.Conv_JsonValueToString` (`BlueprintJsonLibrary.Conv_JsonObjectToJsonValue` _returnvalue "access_token")))
  (if (== Status 200)
    (set `self.AccessToken` _returnvalue_2)
    (set `self.TokenExpiryDateTime` (`BlueprintJsonLibrary.Conv_JsonValueToString` (`BlueprintJsonLibrary.Conv_JsonObjectToJsonValue` _returnvalue "expires_at")))
    (`KismetSystemLibrary.PrintString` _returnvalue_2)
    (else
      (`KismetSystemLibrary.PrintString` "Access Token Not Generated"))))

(event `GetMyIP`
  (bind _whatsmyip (`self.WhatsMyIP`))
  (bind _returnvalue (`|GenericCreateObject` "/Script/WhatsMyPublicIP.WhatsMyPublicIP"))
  (set `self.WhatsMyIP` _returnvalue)
  (`WhatsMyPublicIP.GetMyPublicIP` _whatsmyip)
  (add `WhatsMyPublicIP.OnIPAddressReceived` _whatsmyip (delegate `OnIPAddressRecieverHandle`)))

(event `OnIPAddressRecieverHandle`
  (params (IP :type String))
  (bind _output_get (set `self.IP` IP))
  (`KismetSystemLibrary.PrintString` (`KismetStringLibrary.Concat_StrStr` "My IP Address: " _output_get)))

(event `self.ReceiveInit`
  (bind _returnvalue (`GameplayStatics.GetPlayerController` 0))
  (bind _returnvalue_2 (subsystem `One_Click_EOS_Subsystem`))
  (`self.GetMyIP`)
  (if (`KismetSystemLibrary.IsDedicatedServer`)
    (`self.GetAccessToken`)
    (else
      (`KismetSystemLibrary.Delay` 5.0)
      (`One_Click_EOS_Subsystem.Login_With_EOS` _returnvalue_2 "123" "" "deviceId")
      (if (`KismetSystemLibrary.IsLoggedIn` _returnvalue) :!label _label
        (bind _asbp_player_ctrler (cast `/Game/Creatospace/Blueprints/BP_PlayerCtrler` _returnvalue))
        (`MPGPlayerController.ManageNewPlayer` _asbp_player_ctrler _returnvalue)
        (bind _returnvalue_3 (`One_Click_EOS_Subsystem.getPUID` _returnvalue_2))
        (set `self.PUID` _returnvalue_3)
        (else
          (`KismetSystemLibrary.Delay` 1.0)
          (goto _label))))))

(event `SetRoomObject`
  (params (`RoomObject In` :type "BlueprintJsonObject Structure"))
  (set `self.Room Object` `RoomObject In`))

(event `EnterMP_Server`
  (params (RoomID :type String) (MapName :type String))
  (set `self.Map Name` MapName)
  (bind _output_get (set `self.Room ID` RoomID))
  (`HTTPRequestClient.MakeAHttpRequest` "POST" "https://l49xee5mw4.execute-api.ap-south-1.amazonaws.com/mp-test/startsession" (`|MakeMap` "") (`|MakeMap` "Content-Type" "application/json") (`BlueprintJsonLibrary.Conv_JsonObjectToString` (`BlueprintJsonLibrary.JsonMakeField` (`BlueprintJsonLibrary.JsonMake`) "roomid" (`BlueprintJsonLibrary.JsonMakeString` _output_get))) (delegate `OnSessionCreated`)))

(event `OnSessionCreated`
  (params (Status :type Byte) (ResponseString :type String))
  (`KismetSystemLibrary.PrintString` ResponseString true true (struct :`R` 1.0 :`G` 0.943203 :`A` 1.0))
  (bind _returnvalue (`HTTPRequestClient.ResponseStringToJSON` ResponseString))
  (bind _returnvalue_2 (`HTTPRequestClient.GetObjectFromJSONObject` _returnvalue "PlayerSession"))
  (bind _returnvalue_3 (`HTTPRequestClient.GetStringFromJSONObject` _returnvalue_2 "PlayerSessionId"))
  (set `self.PlayerSession ID` _returnvalue_3)
  (bind _returnvalue_4 (`HTTPRequestClient.GetStringFromJSONObject` _returnvalue_2 "IpAddress"))
  (bind _returnvalue_5 (`HTTPRequestClient.GetStringFromJSONObject` _returnvalue_2 "Port"))
  (bind _returnvalue_6 (`KismetStringLibrary.Concat_StrStr` _returnvalue_4 ":" _returnvalue_5))
  (`KismetSystemLibrary.PrintString` _returnvalue_6)
  (set `self.Server IP Address` _returnvalue_6)
  (`GameplayStatics.OpenLevel` (`KismetStringLibrary.Conv_StringToName` _returnvalue_6)))

(fn `BP_MPGameInstance_AutoGenFunc`
  (returns (ReturnValue :type Boolean))
  (return true))

(fn `GetDatabase`
  (returns (`Mongo Pool` :type "MongoPool Object Reference"))
  (return (`self.Mongo Pool`)))

(fn `GetServerIPAddress`
  (params (MapName :type String))
  (returns (`ServerIP Address` :type String))
  (if (`KismetStringLibrary.EqualEqual_StrStr` MapName "memeRoom")
    (set `self.Server IP Address` "")
    (return (`self.Server IP Address`))
    (elif (`KismetStringLibrary.EqualEqual_StrStr` MapName "exhibition")
      (set `self.Server IP Address` "")
      (return (`self.Server IP Address`))
      (elif (`KismetStringLibrary.EqualEqual_StrStr` MapName "park")
        (set `self.Server IP Address` "")
        (return (`self.Server IP Address`))
        (elif (`KismetStringLibrary.EqualEqual_StrStr` MapName "videoRoom")
          (set `self.Server IP Address` "")
          (return (`self.Server IP Address`))
          (elif (`KismetStringLibrary.EqualEqual_StrStr` MapName "gallery")
            (set `self.Server IP Address` "")
            (return (`self.Server IP Address`))))))))

(fn `GoToLevel`
  (params (mapName :type String))
  (if (`KismetStringLibrary.EqualEqual_StrStr` mapName "memeRoom")
    (`GameplayStatics.OpenLevel` "MemeStreet" true "listen")
    (return)
    (elif (`KismetStringLibrary.EqualEqual_StrStr` mapName "exhibition")
      (`GameplayStatics.OpenLevel` "Auditoriun" true "listen")
      (return)
      (elif (`KismetStringLibrary.EqualEqual_StrStr` mapName "park")
        (`GameplayStatics.OpenLevel` "MeetupPark" true "listen")
        (return)
        (elif true
          (`GameplayStatics.OpenLevel` "VideoRoom" true "listen")
          (return))))))