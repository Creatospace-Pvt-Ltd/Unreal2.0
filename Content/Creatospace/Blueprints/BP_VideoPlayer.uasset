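; Video player actor that streams a room's billboard or flex video and lets players open a Video Player UI.
; ActivateMediaSource reads the first billboard or flex link, chosen by IsBillboard, from the game instance's room JSON, then opens it on the media player and binds the media sound.
; A trigger box stores the overlapping character and shows a prompt; InteractE toggles that character's file-upload UI, and leaving resets the interaction.
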(event `ActivateMediaSource`
  ;[0 0.01784 0.09687] Activate Media Source
  (bind (_mediaplayerout _mediasourceout) (`self.GetMediaSource` (`self.isBillboard`)))
  (bind _returnvalue (`MediaPlayer.OpenSourceWithOptions` _mediaplayerout _mediasourceout (make `MediaPlayerOptions` (struct :`Caption` -1 :`Metadata` -1 :`Script` -1 :`Subtitle` -1 :`Text` -1) "+00000000.00:00:00.000000000" (`self.Play Onload`) (`self.Loop Source`))))
  (if _returnvalue
    (`MediaSoundComponent.SetMediaPlayer` (`self.MediaSound`) _mediaplayerout)
    (else
      (`KismetSystemLibrary.PrintString` "Unable to load source video"))))

(event `self.Box.OnComponentBeginOverlap`
  (params (OverlappedComponent :type "PrimitiveComponent Object Reference") (OtherActor :type "Actor Object Reference") (OtherComp :type "PrimitiveComponent Object Reference") (OtherBodyIndex :type Integer) (bFromSweep :type Boolean) (SweepResult :type "HitResult Structure (by ref)"))
  ;[0.1344 0.1344 0.1344] On Trigger
  (bind _asbp_rpm_third_person_char (cast `/Game/Creatospace/Blueprints/BP_RPM_ThirdPersonChar` OtherActor))
  (bind _output_get (set `self.InteractingActorRef` _asbp_rpm_third_person_char))
  (`/Game/Creatospace/Blueprints/BP_RPM_ThirdPersonChar.Set Custom Text To Viewport` _output_get "Press '" "E" "' to open Video Player UI" "Visible")
  (`/Game/Creatospace/Blueprints/BP_RPM_ThirdPersonChar.Set Custom Text To Viewport` _asbp_rpm_third_person_char "Press '" "E" "' to open Video Player UI" "Visible"))

(event `self.Box.OnComponentEndOverlap`
  (params (OverlappedComponent :type "PrimitiveComponent Object Reference") (OtherActor :type "Actor Object Reference") (OtherComp :type "PrimitiveComponent Object Reference") (OtherBodyIndex :type Integer))
  ;[0.1344 0.1344 0.1344] On Trigger
  (bind _asbp_rpm_third_person_char (cast `/Game/Creatospace/Blueprints/BP_RPM_ThirdPersonChar` OtherActor))
  (`/Game/Creatospace/Blueprints/BP_RPM_ThirdPersonChar.Set Custom Text To Viewport` _asbp_rpm_third_person_char "Creatospace" "None" "" "Visible")
  (`/Game/Creatospace/Blueprints/Interfaces/InteractInterface.ResetInteraction` _asbp_rpm_third_person_char)
  (set `self.currentlyInteracting` false)
  (set `self.InteractingActorRef` null))

(event `/Game/Creatospace/Blueprints/Interfaces/InteractInterface.Interact_E`
  (bind _interactingactorref (`self.InteractingActorRef`))
  ;[1 0.249 0.249] Interact Event
  (if (`self.currentlyInteracting`)
    (set `self.currentlyInteracting` false)
    (`/Engine/EditorBlueprintResources/StandardMacros.IsValid` _interactingactorref
      (:`Is Valid`
        (`/Game/Creatospace/Blueprints/BP_RPM_ThirdPersonChar.doFileUpload` _interactingactorref "Hidden" false)
        (`/Game/Creatospace/Blueprints/BP_RPM_ThirdPersonChar.Set Custom Text To Viewport` _interactingactorref "Press '" "E" "' to open Video Player UI" "Visible")))
    (else
      (set `self.currentlyInteracting` true)
      (`/Engine/EditorBlueprintResources/StandardMacros.IsValid` _interactingactorref
        (:`Is Valid`
          (`/Game/Creatospace/Blueprints/BP_RPM_ThirdPersonChar.doFileUpload` _interactingactorref "Visible" true)
          (`/Game/Creatospace/Blueprints/BP_RPM_ThirdPersonChar.Set Custom Text To Viewport` _interactingactorref "Press 'X" "None" "' to close Video Player UI" "Visible"))))))

(fn `GetMediaSource`
  (params (isBillboard :type Boolean))
  (returns (MediaPlayerOut :type "MediaPlayer Object Reference") (MediaSourceOut :type "MediaSource Object Reference"))
  (locals (StreamURL :type String :default "https://docs.unrealengine.com/5.1/Attachments/working-with-media/integrating-media/MediaFramework/HowTo/FileMediaSource/SampleVideo.mp4"))
  (bind _streamsource (`self.StreamSource`))
  (bind _streamsource_2 (`self.StreamSource`))
  (bind _mediaplayer (`self.MediaPlayer`))
  (`SubmixEffectDelayStatics.SetDelayLength` (make `SubmixEffectDelaySettings` 2000.0) 5.0)
  (bind _asbp_mpgame_instance (cast `/Game/Creatospace/Blueprints/BP_MPGameInstance` (`GameplayStatics.GetGameInstance`))
    (:`then`
      (bind _output_get (set `self.RoomObject` (`BlueprintJsonLibrary.Conv_StringToJsonObject` (`/Game/Creatospace/Blueprints/BP_MPGameInstance.RoomObjectJSON` _asbp_mpgame_instance))))
      (`KismetSystemLibrary.PrintString` (`BlueprintJsonLibrary.Conv_JsonObjectToString` _output_get) false true (struct :`R` 1.0 :`G` 0.806662 :`A` 1.0) 4.0)
      (if isBillboard
        (bind _returnvalue (`BlueprintJsonLibrary.Conv_JsonObjectToJsonValue` _output_get "billboard"))
        (bind _returnvalue_2 (`BlueprintJsonLibrary.Conv_JsonValueToArray` _returnvalue))
        (bind _returnvalue_3 (`BlueprintJsonLibrary.JsonIsNull` _returnvalue))
        (`KismetSystemLibrary.PrintString` (`KismetStringLibrary.Conv_IntToString` (`KismetArrayLibrary.Array_Length` _returnvalue_2)) false _returnvalue_3 (struct :`R` 1.0 :`G` 0.494118 :`A` 1.0) 5.0)
        (if (not _returnvalue_3)
          (bind _returnvalue_4 (`BlueprintJsonLibrary.Conv_JsonValueToString` (`BlueprintJsonLibrary.Conv_JsonObjectToJsonValue` (`BlueprintJsonLibrary.Conv_JsonValueToObject` (`|GetArrayItem` _returnvalue_2)) "link")))
          (set `StreamMediaSource.StreamUrl` _returnvalue_4 _streamsource_2)
          (`KismetSystemLibrary.PrintString` (`KismetStringLibrary.Concat_StrStr` "Billboard>>>" _returnvalue_4) false))
        (else
          (bind _returnvalue_5 (`BlueprintJsonLibrary.Conv_JsonObjectToJsonValue` _output_get "flex"))
          (bind _returnvalue_6 (`BlueprintJsonLibrary.Conv_JsonValueToArray` _returnvalue_5))
          (bind _returnvalue_7 (`BlueprintJsonLibrary.JsonIsNull` _returnvalue_5))
          (`KismetSystemLibrary.PrintString` (`KismetStringLibrary.Conv_IntToString` (`KismetArrayLibrary.Array_Length` _returnvalue_6)) _returnvalue_7 _returnvalue_7 (struct :`R` 1.0 :`G` 0.494118 :`A` 1.0) 5.0)
          (if (not _returnvalue_7)
            (bind _returnvalue_8 (`BlueprintJsonLibrary.Conv_JsonValueToString` (`BlueprintJsonLibrary.Conv_JsonObjectToJsonValue` (`BlueprintJsonLibrary.Conv_JsonValueToObject` (`|GetArrayItem` _returnvalue_6)) "link")))
            (set `StreamMediaSource.StreamUrl` _returnvalue_8 _streamsource_2)
            (`KismetSystemLibrary.PrintString` (`KismetStringLibrary.Concat_StrStr` "Flex>>>" _returnvalue_8) false)))))
    (:`CastFailed`
      (`KismetSystemLibrary.PrintString` "Cast to BP_MPGameInstance Failed in Video Player" false true (struct :`R` 1.0 :`G` 0.079394 :`A` 1.0) 4.0)))
  (bind _output_get_2 (set `StreamMediaSource.StreamUrl` (`MediaSource.GetUrl` _streamsource) _streamsource))
  (`KismetSystemLibrary.PrintString` _output_get_2 false true (struct :`R` 0.957508 :`G` 1.0 :`B` 0.99199 :`A` 1.0) 5.0)
  (bind _returnvalue_9 (`MediaPlayer.CanPlaySource` _mediaplayer _streamsource))
  (if _returnvalue_9
    (`KismetSystemLibrary.PrintString` "Can Play Source" false)
    (else
      (`KismetSystemLibrary.PrintString` "Cannot Play Source" false)))
  (return _mediaplayer _streamsource))

(fn `Set Custom Text To Viewport`
  (params (Prefic :type String) (NewParam2 :type "Key Structure" :default "None") (NewParam3 :type String) (NewParam4 :type "ESlateVisibility Enum" :default "Visible") (Prefix :type String) (`Input Key` :type "Key Structure" :default "None") (Suffix :type String)))

(fn `UserConstructionScript`)