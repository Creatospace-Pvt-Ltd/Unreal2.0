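; Base actor for placeable 3D assets: interacting makes the player character its owner and opens that player's asset widget as selector (Base) or editor (Placeholder, Gizmo).
; Bound widget events toggle the gizmo, store the asset ID and edit the Placeholder's transform.
; Edits route through the owning character, with server and multicast events applying the relative transform.
; glTF URL loading and MongoDB ID saving are unwired.
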(event `self.ReceiveBeginPlay`
  (`self.onToggleGizmo` false)
  (`self.UpdatePlaceholder` "/Game/LevelPrototyping/Meshes/SM_ChamferCube.SM_ChamferCube")
  (`KismetSystemLibrary.Delay` 3.0)
  (`self.UpdatePlaceholder` "/Game/StarterContent/Shapes/Shape_TriPyramid.Shape_TriPyramid"))

(event `/Game/Creatospace/Blueprints/Interfaces/InteractInterface.Interact_E`
  (params (`Actor Ref` :type "Actor Object Reference") (`Component Ref` :type "PrimitiveComponent Object Reference"))
  (bind _placeholder (`self.Placeholder`))
  (bind _defaulttransform (`self.DefaultTransform`))
  (bind _currentwidget (`self.CurrentWidget`))
  ;[0.01298 0.02315 0.1248] Interaction Implementation
  (`|ExecutionSequence`
    (:`then_0`
      (bind _asbp_rpm_third_person_char (cast `/Game/Creatospace/Blueprints/BP_RPM_ThirdPersonChar` `Actor Ref`))
      (`/Game/Creatospace/Blueprints/BP_RPM_ThirdPersonChar.Update Owner SERVER` _asbp_rpm_third_person_char self _asbp_rpm_third_person_char))
    (:`then_1`
      (bind _output_get (set `self.CurrentInteractingActor` `Actor Ref`))
      (bind _asbp_rpm_third_person_char_2 (cast `/Game/Creatospace/Blueprints/BP_RPM_ThirdPersonChar` _output_get))
      (bind _output_get_2 (set `self.CurrentWidget` (`/Game/Creatospace/Blueprints/BP_RPM_ThirdPersonChar.AssetWidget` _asbp_rpm_third_person_char_2)))
      (`WidgetBlueprintLibrary.SetInputMode_GameAndUIEx` (`/Game/Creatospace/Blueprints/BP_RPM_ThirdPersonChar.Current Player Controller` _asbp_rpm_third_person_char_2) _output_get_2)
      (`self.Bind Widget Events` _output_get_2)
      (switch `string` (`KismetSystemLibrary.GetObjectName` `Component Ref`)
        (:`Base`
          (`/Game/Creatospace/Widgets/AssetWidget/WBP_AssetManager.OpenSelector` _currentwidget)
          (`/Game/Creatospace/Widgets/AssetWidget/WBP_AssetManager.SetAssetDetails` _currentwidget _placeholder _defaulttransform))
        (:`Placeholder`
          (`/Game/Creatospace/Widgets/AssetWidget/WBP_AssetManager.OpenEditor` _currentwidget :!label _label)
          (`/Game/Creatospace/Widgets/AssetWidget/WBP_AssetManager.SetAssetDetails` _currentwidget _placeholder _defaulttransform))
        (:`Gizmo`
          (goto _label))))))

(event `/Game/Creatospace/Blueprints/Interfaces/InteractInterface.ResetInteraction`
  ;[0.01298 0.02315 0.1248] Interaction Implementation
  (`|ExecutionSequence`
    (:`then_0`
      (bind _asbp_rpm_third_person_char (cast `/Game/Creatospace/Blueprints/BP_RPM_ThirdPersonChar` (`self.CurrentInteractingActor`)))
      (`/Game/Creatospace/Blueprints/BP_RPM_ThirdPersonChar.Update Owner SERVER` _asbp_rpm_third_person_char self null))
    (:`then_1`
      (bind _currentwidget (`self.CurrentWidget`)
        (:`then`
          (`/Game/Creatospace/Widgets/AssetWidget/WBP_AssetManager.CloseWidget` _currentwidget))
        (:`else`)))))

(event `UpdatePlaceholder`
  (params (`New Static Mesh` :type "StaticMesh Object Reference"))
  (bind _placeholder (`self.Placeholder`))
  (bind (_returnvalue_x _returnvalue_y _returnvalue_z) (`KismetMathLibrary.BreakVector` (`SceneComponent.K2_GetComponentLocation` (`self.Base`))))
  (bind (_min _max) (break `Box` (`StaticMesh.GetBoundingBox` (`StaticMeshComponent.StaticMesh` _placeholder))))
  (bind (_returnvalue_x_2 _returnvalue_y_2 _returnvalue_z_2) (`KismetMathLibrary.BreakVector` (- _max _min)))
  ;[0.149 0 0.1529] Update Placeholder Mesh
  (`StaticMeshComponent.SetStaticMesh` (`self.Placeholder`) `New Static Mesh`)
  (`SceneComponent.K2_SetWorldLocation` _placeholder (`KismetMathLibrary.MakeVector` _returnvalue_x _returnvalue_y (+ (* _returnvalue_z_2 0.5) _returnvalue_z 50.0)) false false)
  (bind _output_get (set `self.DefaultTransform` (`SceneComponent.K2_GetComponentToWorld` _placeholder)))
  (bind _currentwidget (`self.CurrentWidget`)
    (:`then`
      (`/Game/Creatospace/Widgets/AssetWidget/WBP_AssetManager.SetAssetDetails` _currentwidget (`self.Placeholder`) _output_get))
    (:`else`)))

(event `Bind Widget Events`
  (params (`Asset Widget Ref` :type "/Game/Creatospace/Widgets/AssetWidget/WBP_AssetManager Object Reference"))
  (`|ExecutionSequence`
    (:`then_0`
      ;[0.149 0 0.1529] Gizmo
      (add `/Game/Creatospace/Widgets/AssetWidget/WBP_AssetManager.onToggleGizmo` `Asset Widget Ref` (delegate `onToggleGizmo`)))
    (:`then_1`
      ;[0.01298 0.02315 0.1248] Asset ID Change from URL
      (add `/Game/Creatospace/Widgets/AssetWidget/WBP_AssetManager.onAsset ID Changed` `Asset Widget Ref` (delegate `onAssetIDChanged`)))
    (:`then_2`
      ;[0 0.3864 0.8148] Location Change Applied
      (add `/Game/Creatospace/Widgets/AssetWidget/WBP_AssetManager.onLocationChanged` `Asset Widget Ref` (delegate `onLocationChanged`)))
    (:`then_3`
      ;[0.001518 0.1384 0.4342] Rotation Changed Applied
      (add `/Game/Creatospace/Widgets/AssetWidget/WBP_AssetManager.onRotationChanged` `Asset Widget Ref` (delegate `onRotationChanged`)))
    (:`then_4`
      ;[0.01298 0.02315 0.1248] Scale Change Applied
      (add `/Game/Creatospace/Widgets/AssetWidget/WBP_AssetManager.onScaleChanged` `Asset Widget Ref` (delegate `onScaleChanged`)))))

(event `onToggleGizmo`
  (params (isVisible :type Boolean) (isActive :type Boolean))
  (bind _gizmo (`self.Gizmo`))
  ;[0.149 0 0.1529] Gizmo
  (`SceneComponent.SetVisibility` _gizmo isVisible false)
  (`ActorComponent.SetActive` _gizmo isActive false))

(event `onAssetIDChanged`
  (params (`New 3DAsset ID` :type String))
  ;[0.01298 0.02315 0.1248] Asset ID Change from URL
  (bind _output_get (set `self.Current3DAssetID` `New 3DAsset ID`))
  (`KismetSystemLibrary.PrintString` (`KismetStringLibrary.Concat_StrStr` "NEW ASSET ID SET: " _output_get)))

(event `OnAssetLoaded`
  (params (Asset :type "glTFRuntimeAsset Object Reference"))
  (bind _placeholder (`self.Placeholder`))
  (bind _placeholder_2 (`self.Placeholder`))
  ;[0.01298 0.02315 0.1248] Asset ID Change from URL
  (bind _returnvalue (`|SpawnActorFromClass` "/Script/glTFRuntime.glTFRuntimeAssetActor" (`SceneComponent.K2_GetComponentToWorld` _placeholder) "Undefined" "OverrideRootScale" null Asset (make `glTFRuntimeStaticMeshConfig` :`Outer` _placeholder) (struct) (struct) true false true true null))
  (`self.K2_AttachToComponent` _returnvalue _placeholder_2 "None" "SnapToTarget" "SnapToTarget" "SnapToTarget" true)
  (`StaticMeshComponent.SetStaticMesh` _placeholder_2 null))

(event `onLocationChanged`
  (params (`Location Axis Name` :type "ERigControlAxis Enum" :default "X") (`New Value` :type "Float (double-precision)"))
  (bind _returnvalue (* `New Value` 100.0))
  (bind _defaulttransform (`self.DefaultTransform`))
  (bind _placeholder (`self.Placeholder`))
  (bind (_returnvalue_x _returnvalue_y _returnvalue_z) (`KismetMathLibrary.BreakVector` (`SceneComponent.K2_GetComponentLocation` _placeholder)))
  ;[0 0.3864 0.8148] Location Change Applied
  (switch `ERigControlAxis` `Location Axis Name`
    (:`X`
      (`SceneComponent.K2_SetWorldLocation` _placeholder (`KismetMathLibrary.MakeVector` (+ _returnvalue (.x (.location _defaulttransform))) _returnvalue_y _returnvalue_z) true false))
    (:`Y`
      (`SceneComponent.K2_SetWorldLocation` _placeholder (`KismetMathLibrary.MakeVector` _returnvalue_x (+ (.y (.location _defaulttransform)) _returnvalue) _returnvalue_z) true false))
    (:`Z`
      (`SceneComponent.K2_SetWorldLocation` _placeholder (`KismetMathLibrary.MakeVector` _returnvalue_x _returnvalue_y (+ (.z (.location _defaulttransform)) _returnvalue)) true false)))
  (`self.Update Transform Local`))

(event `onRotationChanged`
  (params (`Rotation Axis Name` :type "ERigControlAxis Enum" :default "X") (`New Value` :type "Float (double-precision)"))
  (bind _returnvalue (* `New Value` 360.0))
  (bind _placeholder (`self.Placeholder`))
  (bind (_relativerotation_roll _relativerotation_pitch _relativerotation_yaw) (`KismetMathLibrary.BreakRotator` (`SceneComponent.RelativeRotation` _placeholder)))
  ;[0.001518 0.1384 0.4342] Rotation Changed Applied
  (switch `ERigControlAxis` `Rotation Axis Name`
    (:`X`
      (`SceneComponent.K2_SetRelativeRotation` _placeholder (`KismetMathLibrary.MakeRotator` _returnvalue _relativerotation_pitch _relativerotation_yaw) false false))
    (:`Y`
      (`SceneComponent.K2_SetRelativeRotation` _placeholder (`KismetMathLibrary.MakeRotator` _relativerotation_roll _returnvalue _relativerotation_yaw) false false))
    (:`Z`
      (`SceneComponent.K2_SetRelativeRotation` _placeholder (`KismetMathLibrary.MakeRotator` _relativerotation_roll _relativerotation_pitch _returnvalue) false false)))
  (`self.Update Transform Local`))

(event `onScaleChanged`
  (params (`Scale Axis Name` :type "ERigControlAxis Enum" :default "X") (`New Value` :type "Float (double-precision)"))
  (bind _placeholder (`self.Placeholder`))
  (bind (_returnvalue_x _returnvalue_y _returnvalue_z) (`KismetMathLibrary.BreakVector` (`SceneComponent.K2_GetComponentScale` _placeholder)))
  ;[0.01298 0.02315 0.1248] Scale Change Applied
  (switch `ERigControlAxis` `Scale Axis Name`
    (:`X`
      (`SceneComponent.SetWorldScale3D` _placeholder (`KismetMathLibrary.MakeVector` `New Value` _returnvalue_y _returnvalue_z)))
    (:`Y`
      (`SceneComponent.SetWorldScale3D` _placeholder (`KismetMathLibrary.MakeVector` _returnvalue_x `New Value` _returnvalue_z)))
    (:`Z`
      (`SceneComponent.SetWorldScale3D` _placeholder (`KismetMathLibrary.MakeVector` _returnvalue_x _returnvalue_y `New Value`))))
  (`self.Update Transform Local`))

(event `Update Transform Local`
  ;[0.9028 0.1796 0.9219] Replication Events
  (bind _asbp_rpm_third_person_char (cast `/Game/Creatospace/Blueprints/BP_RPM_ThirdPersonChar` (`self.GetOwner`)))
  (`/Game/Creatospace/Blueprints/BP_RPM_ThirdPersonChar.Update Asset Transform` _asbp_rpm_third_person_char self (`SceneComponent.GetRelativeTransform` (`self.Placeholder`))))

(event `Update Transform SERVER`
  (params (`Updated Transform` :type "Transform Structure"))
  ;[0.9028 0.1796 0.9219] Replication Events
  (`SceneComponent.K2_SetRelativeTransform` (`self.Placeholder`) `Updated Transform` false false)
  (`KismetSystemLibrary.PrintString` "IN SERVER CALL" true true (struct :`R` 0.14902 :`B` 0.152941 :`A` 1.0) 5.0)
  (`self.Update Transform MULTI` `Updated Transform`))

(event `Update Transform MULTI`
  (params (`Updated Transform` :type "Transform Structure"))
  ;[0.9028 0.1796 0.9219] Replication Events
  (`KismetSystemLibrary.PrintString` "IN MULTICAST CALL" true true (struct :`R` 0.012983 :`G` 0.023153 :`B` 0.124772 :`A` 1.0) 5.0)
  (`SceneComponent.K2_SetRelativeTransform` (`self.Placeholder`) `Updated Transform` false false))

(fn `UserConstructionScript`)