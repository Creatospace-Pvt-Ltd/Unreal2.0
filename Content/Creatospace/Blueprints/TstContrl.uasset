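; Player controller for multiplayer rooms, handling server sessions, map travel, Dolby.io voice, chat and online-member lists.
; Chat and member changes are written to BP_GameState, and rep-notify events update the BP_HUD_General room widgets.
; Session end returns clients to Lobby, and the last player out also terminates the game session.
; Custom possession events switch the view target, and Jump clears sitting animations; avatar-load and LeaveVoiceRoom handlers are stubs.
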(event `set Room id`
  (params (`Room ID` :type String))
  ;[0.01298 0.02315 0.1248] Set IDs
  (set `self.Room ID` `Room ID`))

(event `Print on client`
  (params (String :type String))
  (`KismetSystemLibrary.PrintString` (`KismetStringLibrary.Concat_StrStr` "Print from server: " String)))

(event `Accept my client`
  (params (`Client session id` :type String))
  (`self.AcceptClient` `Client session id`))

(event `set Map name`
  (params (`map name` :type String))
  ;[0.01298 0.02315 0.1248] Set IDs
  (set `self.Map Name` `map name`))

(event `Set Server IP`
  (params (`Server IP` :type String))
  ;[0.01298 0.02315 0.1248] Set IDs
  (set `self.Server IP` `Server IP`))

(event `Server session find`
  (params (Map :type String))
  (`AdvancedSessionsLibrary.ServerTravel` Map true))

(event `Start Voice`
  (bind _asbp_mpgame_instance (cast `/Game/Creatospace/Blueprints/BP_MPGameInstance` (`GameplayStatics.GetGameInstance`)))
  (bind _myuser (`/Game/Creatospace/Blueprints/BP_MPGameInstance.MyUser` _asbp_mpgame_instance))
  (`DolbyIOSubsystem.Connect` (subsystem `DolbyIOSubsystem`) (`/Game/Creatospace/Blueprints/BP_MPGameInstance.Room ID` _asbp_mpgame_instance) (`KismetStringLibrary.Concat_StrStr` (`BlueprintJsonLibrary.Conv_JsonValueToString` (`BlueprintJsonLibrary.Conv_JsonObjectToJsonValue` _myuser "fname")) " " (`BlueprintJsonLibrary.Conv_JsonValueToString` (`BlueprintJsonLibrary.Conv_JsonObjectToJsonValue` _myuser "lname"))) (`/Game/Creatospace/Blueprints/BP_MPGameInstance.User ID` _asbp_mpgame_instance) (`BlueprintJsonLibrary.Conv_JsonValueToString` (`BlueprintJsonLibrary.Conv_JsonObjectToJsonValue` (`BlueprintJsonLibrary.Conv_JsonValueToObject` (`BlueprintJsonLibrary.Conv_JsonObjectToJsonValue` _myuser "profImg")) "link")) "Active" "Shared"))

(event `Leave VoiceRoom`
  ;[0.2971 1 0.9202] Leave voice Room
  (bind _asbp_mpgame_instance (cast `/Game/Creatospace/Blueprints/BP_MPGameInstance` (`GameplayStatics.GetGameInstance`))))

(event `Mute`
  (`DolbyIOSubsystem.MuteInput` (subsystem `DolbyIOSubsystem`)))

(event `OpenChatSystem`
  (bind _chatboxwidget (`self.ChatBoxWidget`))
  ;[0.149 0 0.1529] Mute / Unmute
  (if (`self.Is Chat Visible`)
    (`Widget.SetVisibility` _chatboxwidget "Hidden")
    (set `self.Is Chat Visible` false)
    (else
      (`Widget.SetVisibility` _chatboxwidget "Visible")
      (set `self.Is Chat Visible` true))))

(event `self.ReceiveBeginPlay`
  ;[0.5906 0.03467 0.6052] For Avatar change
  (bind _returnvalue (`|CreateWidget` "/Game/Creatospace/Widgets/WBP_AvatarConfig.WBP_AvatarConfig_C" (`GameplayStatics.GetPlayerController` 0)))
  (set `self.WBP_AvatarConfig` _returnvalue)
  (cast `ExampleCharacter` (`self.K2_GetPawn` (`GameplayStatics.GetPlayerController` 0)))
  (add `/Game/Creatospace/Widgets/WBP_AvatarConfig.AvatarGeneratedEvent` (`self.WBP_AvatarConfig`) (delegate `CallAvatarLoadServer`)))

(event `Unmute`
  (`DolbyIOSubsystem.UnmuteInput` (subsystem `DolbyIOSubsystem`)))

(event `CallAvatarLoadServer`
  (params (AvatarUrl :type String))
  ;[0.5906 0.03467 0.6052] For Avatar change
)

(event `Server AddMessage`
  (params (User :type String) (Message :type Text))
  (bind _returnvalue (`BlueprintJsonLibrary.Conv_StringToJsonObject` User))
  ;[0.001518 0.1384 0.4342] Server Add Message / User
  (bind _asbp_game_state (cast `/Game/Creatospace/Blueprints/BP_GameState` (`GameplayStatics.GetGameState`)))
  (`/Game/Creatospace/Blueprints/BP_GameState.AddMessage` _asbp_game_state (make `/Game/Creatospace/Widgets/SMessageData` _returnvalue Message (`KismetTextLibrary.AsTimeZoneDate_DateTime` (`KismetMathLibrary.GetDate` (`KismetMathLibrary.UtcNow`)))))
  (`self.Print on client` (`BlueprintJsonLibrary.Conv_JsonObjectToString` _returnvalue)))

(event `Client travel called from server`
  (params (Map :type String))
  (`GameplayStatics.OpenLevel` (`KismetStringLibrary.Conv_StringToName` Map)))

(event `End Server session`
  (params (`Player Session ID` :type String))
  (bind _returnvalue (`GameplayStatics.GetNumPlayerControllers`))
  (`self.Print on client` (`KismetStringLibrary.Conv_IntToString` _returnvalue))
  (if (== _returnvalue 1)
    (`KismetSystemLibrary.Delay` 0.2)
    (`self.Client travel called from server` "Lobby")
    (`GameplayStatics.OpenLevel` "Server")
    (`KismetSystemLibrary.Delay` 1.0)
    (`self.TerminateGameSession`)
    (else
      (`self.Client travel called from server` "Lobby")
      (`self.RemovePlayerSession` `Player Session ID`))))

(event `Server add Online User`
  (params (`User ID` :type String) (`User JSON` :type String))
  (bind _returnvalue (`BlueprintJsonLibrary.Conv_StringToJsonObject` `User JSON`))
  ;[0.001518 0.1384 0.4342] Server Add Message / User
  (bind _asbp_game_state (cast `/Game/Creatospace/Blueprints/BP_GameState` (`GameplayStatics.GetGameState`)))
  (`/Game/Creatospace/Blueprints/BP_GameState.Add Online Member` _asbp_game_state (make `/Game/Creatospace/Widgets/OnlineUser` `User ID` _returnvalue))
  (`self.Print on client` (`BlueprintJsonLibrary.Conv_JsonObjectToString` _returnvalue)))

(event `Server Remove Online User`
  (params (`User ID` :type String))
  ;[0.001518 0.1384 0.4342] Server Add Message / User
  (bind _asbp_game_state (cast `/Game/Creatospace/Blueprints/BP_GameState` (`GameplayStatics.GetGameState`)))
  (`/Game/Creatospace/Blueprints/BP_GameState.Remove  Online Member` _asbp_game_state `User ID`)
  (`self.Print on client` `User ID`))

(event `OnRepNotifyClient`
  (params (`User ID` :type String) (`User JSON` :type String))
  ;[0.01298 0.02315 0.1248] On Rep Notify
  (`KismetSystemLibrary.PrintString` `User JSON`)
  (bind _asbp_hud_general (cast `/Game/Creatospace/Widgets/BP_HUD_General` (`self.GetHUD`)))
  (`/Game/Creatospace/Widgets/WBP_OnlineMembers.Add Online User` (`/Game/Creatospace/Widgets/BP_RoomWidget.Online Members Widget` (`/Game/Creatospace/Widgets/BP_HUD_General.Room Widget` _asbp_hud_general)) (make `/Game/Creatospace/Widgets/OnlineUser` `User ID` (`BlueprintJsonLibrary.Conv_StringToJsonObject` `User JSON`))))

(event `OnRepNotifyMessage`
  (params (Message :type String) (`User JSON` :type String) (Time :type Text))
  ;[0.01298 0.02315 0.1248] On Rep Notify
  (`KismetSystemLibrary.PrintString` `User JSON`)
  (bind _asbp_hud_general (cast `/Game/Creatospace/Widgets/BP_HUD_General` (`self.GetHUD`)))
  (`/Game/Creatospace/Widgets/WBP_ChatBox.AddmessageEntry` (`/Game/Creatospace/Widgets/BP_RoomWidget.Chat Box Widget` (`/Game/Creatospace/Widgets/BP_HUD_General.Room Widget` _asbp_hud_general)) (make `/Game/Creatospace/Widgets/SMessageData` (`BlueprintJsonLibrary.Conv_StringToJsonObject` `User JSON`) (`KismetTextLibrary.Conv_StringToText` Message) Time)))

(event `End Voice`
  (`DolbyIOSubsystem.Disconnect` (subsystem `DolbyIOSubsystem`)))

(event `OnRepNotifyRemoveMember`
  (params (`User ID` :type String))
  ;[0.01298 0.02315 0.1248] On Rep Notify
  (`KismetSystemLibrary.PrintString` `User ID`)
  (bind _asbp_hud_general (cast `/Game/Creatospace/Widgets/BP_HUD_General` (`self.GetHUD`)))
  (`/Game/Creatospace/Widgets/WBP_OnlineMembers.Remove Online Member` (`/Game/Creatospace/Widgets/BP_RoomWidget.Online Members Widget` (`/Game/Creatospace/Widgets/BP_HUD_General.Room Widget` _asbp_hud_general)) `User ID`))

(event `self.ReceivePossess`
  (params (PossessedPawn :type "Pawn Object Reference"))
  ;[0.001518 0.1384 0.4342] Custom Possession flow
  (`self.SetViewTargetWithBlend` PossessedPawn))

(event `self.ReceiveUnPossess`
  (params (UnpossessedPawn :type "Pawn Object Reference"))
  ;[0.001518 0.1384 0.4342] Custom Possession flow
  (`self.SetViewTargetWithBlend` UnpossessedPawn)
  (`KismetSystemLibrary.Delay` 1.0)
  (set `self.Unpossessed Pawn` null))

(event `InputAction|Jump`
  (params (Key :type "Key Structure"))
  (bind _returnvalue (`self.K2_GetPawn`))
  ;[0.01298 0.02315 0.1248] Jump Action Rebinding for Animations
  (:`Pressed`
    (`/Engine/EditorBlueprintResources/StandardMacros.DoOnce` false :!label _label
      (:`Completed`
        (`/Engine/EditorBlueprintResources/StandardMacros.IsValid` _returnvalue
          (:`Is Valid`
            (bind _asbp_rpm_third_person_char (cast `/Game/Creatospace/Blueprints/BP_RPM_ThirdPersonChar` _returnvalue))
            (if (`/Game/Creatospace/Blueprints/BP_RPM_ThirdPersonChar.isSitting` _asbp_rpm_third_person_char)
              (message `/Game/Creatospace/Blueprints/Interfaces/AnimationInterface.ClearAnimation` _asbp_rpm_third_person_char)
              (`KismetSystemLibrary.Delay` 3.0 :!label _label_2)
              (goto _label :!via `Reset`)
              (else
                (`Character.Jump` _asbp_rpm_third_person_char))))
          (:`Is Not Valid`
            (bind _unpossessed_pawn (`self.Unpossessed Pawn`)
              (:`then`
                (message `/Game/Creatospace/Blueprints/Interfaces/AnimationInterface.ClearAnimation` _unpossessed_pawn)
                (goto _label_2))
              (:`else`))))))))

(fn `UserConstructionScript`)