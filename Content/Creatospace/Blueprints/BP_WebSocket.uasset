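; BP_WebSocket is an actor that listens to a Socket.IO server through its SocketIOClient component and prints what it receives.
; On BeginPlay it binds the "fetchid" event on the root namespace to the generic event handler.
; The handler prints that event's data, or a mismatch message for any other event name.
; Connection and disconnection, including the reason, are also shown as on-screen debug text; nothing is emitted or stored.
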(event `self.SocketIOClient.OnConnected`
  (params (SocketId :type String) (SessionId :type String) (bIsReconnection :type Boolean))
  (`KismetSystemLibrary.PrintString` "Connected" true true (struct :`G` 1.0 :`B` 0.211438 :`A` 1.0) 15.0))

(event `self.SocketIOClient.OnDisconnected`
  (params (Reason :type "ESIOConnectionCloseReason Enum" :default "CLOSE_REASON_NORMAL"))
  (`KismetSystemLibrary.PrintString` (`KismetStringLibrary.Concat_StrStr` "Disconnected reason: " (`|GetEnumeratorNameAsString` Reason)) true true (struct :`R` 0.010433 :`G` 1.0 :`A` 1.0) 15.0))

(event `self.ReceiveBeginPlay`
  (`SocketIOClientComponent.BindEventToGenericEvent` (`self.SocketIOClient`) "fetchid" "/"))

(event `self.SocketIOClient.OnGenericEvent`
  (params (EventName :type String) (EventData :type "SIOJsonValue Object Reference"))
  (if (== EventName "fetchid")
    (`KismetSystemLibrary.PrintString` (`SIOJLibrary.Conv_SIOJsonValueToString` EventData) true true (struct :`R` 0.020647 :`G` 1.0 :`A` 1.0))
    (else
      (`KismetSystemLibrary.PrintString` (`KismetStringLibrary.Concat_StrStr` "Event mismatched evnt name: " EventName) true true (struct :`G` 1.0 :`B` 0.023826 :`A` 1.0)))))

(fn `UserConstructionScript`)