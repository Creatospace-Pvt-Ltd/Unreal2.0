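; Game state for a Creatospace room, holding the room object, chat message history and online member list.
; Add and remove events run only on a dedicated server, updating the arrays and then calling notify events on player 0's BP_RPM_ThirdPersonChar.
; Both arrays' OnRep functions are empty, so that character alone relays changes here; member removal passes it an empty string rather than the user ID.
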(event `SetRoomObject`
  (params (RoomObject :type "BlueprintJsonObject Structure"))
  (set `self.RoomObject` RoomObject))

(event `AddMessage`
  (params (Message :type "/Game/Creatospace/Widgets/SMessageData Structure"))
  (if (`KismetSystemLibrary.IsDedicatedServer`)
    (`KismetSystemLibrary.PrintString` "AddMessage")
    (`KismetArrayLibrary.Array_Add` (`self.MessagesArray`) (make `/Game/Creatospace/Widgets/SMessageData` Message_User_16_381BCA2A4BCE652885BFE889AA4C0EE4 Message_MessageContent_8_D66B48CC45B579775B9C369F6446FD82 Message_Time_15_D78C947F47D2029E537EFD9D2978A904))
    (bind _asbp_rpm_third_person_char (cast `/Game/Creatospace/Blueprints/BP_RPM_ThirdPersonChar` (`GameplayStatics.GetPlayerCharacter` 0)))
    (`/Game/Creatospace/Blueprints/BP_RPM_ThirdPersonChar.OnRepNotifyMessage` _asbp_rpm_third_person_char (`KismetTextLibrary.Conv_TextToString` Message_MessageContent_8_D66B48CC45B579775B9C369F6446FD82) (`BlueprintJsonLibrary.Conv_JsonObjectToString` Message_User_16_381BCA2A4BCE652885BFE889AA4C0EE4) Message_Time_15_D78C947F47D2029E537EFD9D2978A904)))

(event `Add Online Member`
  (params (user :type "/Game/Creatospace/Widgets/OnlineUser Structure"))
  (bind _returnvalue (`BlueprintJsonLibrary.Conv_JsonObjectToString` user_UserJSON_8_ED935A6448DB7815E987A796B8781E9E))
  (if (`KismetSystemLibrary.IsDedicatedServer`)
    (`KismetArrayLibrary.Array_Add` (`self.MemberList`) (make `/Game/Creatospace/Widgets/OnlineUser` user_UserID_11_81A9F6AA4463CCF365F07082FB34F66A user_UserJSON_8_ED935A6448DB7815E987A796B8781E9E))
    (bind _asbp_rpm_third_person_char (cast `/Game/Creatospace/Blueprints/BP_RPM_ThirdPersonChar` (`GameplayStatics.GetPlayerCharacter` 0)))
    (`/Game/Creatospace/Blueprints/BP_RPM_ThirdPersonChar.OnRepNotifyClient` _asbp_rpm_third_person_char user_UserID_11_81A9F6AA4463CCF365F07082FB34F66A _returnvalue)
    (`/Game/Creatospace/Blueprints/BP_RPM_ThirdPersonChar.Print on client` _asbp_rpm_third_person_char _returnvalue)))

(event `Remove  Online Member`
  (params (`User ID` :type String))
  (bind _memberlist (`self.MemberList`))
  (if (`KismetSystemLibrary.IsDedicatedServer`)
    (for _array_element _memberlist
      (if (`KismetStringLibrary.EqualEqual_StrStr` `User ID` (`.UserID_11_81A9F6AA4463CCF365F07082FB34F66A` (break `/Game/Creatospace/Widgets/OnlineUser` _array_element)))
        (`KismetArrayLibrary.Array_RemoveItem` _memberlist _array_element)))
    (bind _asbp_rpm_third_person_char (cast `/Game/Creatospace/Blueprints/BP_RPM_ThirdPersonChar` (`GameplayStatics.GetPlayerCharacter` 0)))
    (`/Game/Creatospace/Blueprints/BP_RPM_ThirdPersonChar.OnRepNotifyRemoveMember` _asbp_rpm_third_person_char "")))

(fn `GetRoomObject`
  (returns (RoomObject :type "BlueprintJsonObject Structure"))
  (return (`self.RoomObject`)))

(fn `OnRep_MemberList`)

(fn `OnRep_MessagesArray`)

(fn `UserConstructionScript`)