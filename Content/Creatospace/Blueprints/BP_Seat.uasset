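; BP_Seat is an interactable seat that lets the Ready Player Me third-person character sit by pressing E.
; Overlap caches the character and shows the prompt; leaving resets its interaction, text and the seat state.
; A DoOnce gates Sit, which sends the preview animation and collision location to the character.
; GetRevert exposes the revert animation, and DebugMode prints the interaction and seated flags each tick.
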(event `self.ReceiveBeginPlay`)

(event `self.ReceiveTick`
  (params (DeltaSeconds :type "Float (single-precision)"))
  ;[0.149 0 0.1529] Debug Booleans
  (if (`self.DebugMode`)
    (`KismetSystemLibrary.PrintString` (`KismetStringLibrary.Concat_StrStr` "I =" (`KismetStringLibrary.Conv_BoolToString` (`self.Interacting`)) "  ; S=" (`KismetStringLibrary.Conv_BoolToString` (`self.Seated`))) true false (struct :`G` 0.66 :`B` 1.0 :`A` 1.0) DeltaSeconds)))

(event `self.ReceiveActorBeginOverlap`
  (params (OtherActor :type "Actor Object Reference"))
  ;[0.01298 0.02315 0.1248] Overlap Functions & Interaction
  (bind _asbp_rpm_third_person_char (cast `/Game/Creatospace/Blueprints/BP_RPM_ThirdPersonChar` OtherActor))
  (set `self.RPM_TPC_Ref` _asbp_rpm_third_person_char)
  (if true
    (`/Game/Creatospace/Blueprints/BP_RPM_ThirdPersonChar.Set Custom Text To Viewport` _asbp_rpm_third_person_char "Press '" "E" "' to Sit" "Visible")
    (set `self.Interacting` true)))

(event `self.ReceiveActorEndOverlap`
  (params (OtherActor :type "Actor Object Reference"))
  (bind _rpm_tpc_ref (`self.RPM_TPC_Ref`))
  ;[0.01298 0.02315 0.1248] Overlap Functions & Interaction
  (cast `/Game/Creatospace/Blueprints/BP_RPM_ThirdPersonChar` OtherActor)
  (`/Game/Creatospace/Blueprints/BP_RPM_ThirdPersonChar.Set Custom Text To Viewport` _rpm_tpc_ref "Creatospace" "None" "" "Visible")
  (`/Game/Creatospace/Blueprints/Interfaces/InteractInterface.ResetInteraction` _rpm_tpc_ref)
  (set `self.RPM_TPC_Ref` null)
  (if true
    (set `self.Interacting` false)
    (set `self.Seated` false)
    (goto _label :!via `Reset`)))

(event `/Game/Creatospace/Blueprints/Interfaces/InteractInterface.Interact_E`
  (params (`Actor Ref` :type "Actor Object Reference"))
  ;[0.01298 0.02315 0.1248] Overlap Functions & Interaction
  (if (`self.Interacting`)
    (if (not (`self.Seated`))
      (`/Engine/EditorBlueprintResources/StandardMacros.DoOnce` false :!label _label
        (:`Completed`
          (`self.Sit`)
          (set `self.Seated` true)
          (`/Game/Creatospace/Blueprints/BP_RPM_ThirdPersonChar.Set Custom Text To Viewport` (`self.RPM_TPC_Ref`) "Sitting..." "None" "" "Visible"))))))

(fn `GetRevert`
  (returns (RevertAnim :type "AnimSequence Object Reference"))
  (return (`self.RevertAnimation`)))

(fn `Sit`
  (message `/Game/Creatospace/Blueprints/Interfaces/AnimationInterface.TriggerAnimation` (`self.RPM_TPC_Ref`) (`self.PreviewAnim`) (`SceneComponent.K2_GetComponentLocation` (`self.PlayerCollision`)))
  (set `self.Seated` true))

(fn `UserConstructionScript`)